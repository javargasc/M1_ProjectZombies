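; BP_ChargerEnemy is a melee enemy that charges the first-person player on sight and damages them on contact.
; Pawn sensing sends it moving toward a seen FirstPersonCharacter with AI MoveTo, and hitting an actor tagged Player applies a fixed amount of damage.
; Incoming damage reduces its Life, and once that drops below zero it flags itself dead, prints a debug message and destroys itself.
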(event `self.PawnSensing.OnSeePawn`
  (params (Pawn :type "Pawn Object Reference"))
  (bind _asfirst_person_character (cast `/Game/FirstPersonCPP/Blueprints/FirstPersonCharacter` Pawn))
  (`|AIMoveTo` self (0.0 0.0 0.0) _asfirst_person_character))

(event `self.ReceiveAnyDamage`
  (params (Damage :type "Float (single-precision)") (DamageType :type "DamageType Object Reference") (InstigatedBy :type "Controller Object Reference") (DamageCauser :type "Actor Object Reference"))
  (bind _life (`self.Life`))
  (set `self.Life` (- _life Damage))
  (if (< _life 0.0)
    (set `self.isDead` true)
    (`KismetSystemLibrary.PrintString` "I am dead")
    (`self.K2_DestroyActor`)))

(event `self.ReceiveHit`
  (params (MyComp :type "PrimitiveComponent Object Reference") (Other :type "Actor Object Reference") (OtherComp :type "PrimitiveComponent Object Reference") (bSelfMoved :type Boolean) (HitLocation :type "Vector Structure") (HitNormal :type "Vector Structure") (NormalImpulse :type "Vector Structure") (Hit :type "HitResult Structure (by ref)"))
  (if (`self.ActorHasTag` Other "Player")
    (`GameplayStatics.ApplyDamage` Other 50.0)))

(fn `UserConstructionScript`)