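; BP_Health is a health component that tracks a single life value for whatever actor owns it.
; BeginPlay sets the life to full, and ApplyDamage subtracts the given amount from it without clamping.
; GetLife returns the current value, and IsLive reports whether it is still above zero.
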(event `self.ReceiveBeginPlay`
  (set `self.LifeAmount` 100.0))

(fn `ApplyDamage`
  (params (DamageAmount :type "Float (double-precision)"))
  (set `self.LifeAmount` (- (`self.LifeAmount`) DamageAmount)))

(fn `Get Life`
  (returns (Life :type "Float (double-precision)"))
  (return (`self.LifeAmount`)))

(fn `IsLive`
  (returns (IsLive :type Boolean))
  (return (> (`self.LifeAmount`) 0.0)))