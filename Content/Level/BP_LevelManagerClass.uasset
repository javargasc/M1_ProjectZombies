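; Level manager Blueprint that registers itself with C_BP_GameMode on BeginPlay as its LevelManagerCPP.
; Number keys 1 to 4 manually trigger BeginRound, EndRound, Win and Lose, whose logic is not defined in this graph.
; The EnableInput call for player controller 0 is unconnected, and WinNOCPP is an empty stub.
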(event `self.ReceiveBeginPlay`
  (bind _asc_bp_game_mode (cast `/Game/FirstPersonCPP/Blueprints/C_BP_GameMode` (`GameplayStatics.GetGameMode`)))
  (set `C_GameModeBase.LevelManagerCPP` self _asc_bp_game_mode))

(event `Key|One`
  (params (Key :type "Key Structure"))
  (:`Pressed`
    (`self.BeginRound`)))

(event `Key|Two`
  (params (Key :type "Key Structure"))
  (:`Pressed`
    (`self.EndRound`)))

(event `Key|Three`
  (params (Key :type "Key Structure"))
  (:`Pressed`
    (`self.Win`)))

(event `Key|Four`
  (params (Key :type "Key Structure"))
  (:`Pressed`
    (`self.Lose`)))

(fn `UserConstructionScript`)

(fn `Win_NOCPP`)